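; BP_Dispender is a harvestable interactable that dispenses an item to the player, then regrows on a timer.
; Yield, stack, harvest time and damage come from the item's DataTable row at BeginPlay.
; Interact checks any required item via LSBlueprints, adds the yield to the character save, applies damage through the HUD, and sequences animations, sounds and delays until harvestable again.
; A cheat flag skips the item check and shortens the cooldown.
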(event `self.ReceiveBeginPlay`
  (bind (_item_datatable _item_rowname) (break `DataTableRowHandle` (`self.Item`)))
  (set `self.ItemName` _item_rowname)
  (bind _returnvalue (`|GetDataTableRow` _item_datatable _item_rowname)
    (:`then`
      (bind ((`Dispender_2_D898B50D40645906524197A746DA9133` _dispender) (`Stack_4_CE9FA3BA4DDFFEA73CFC659E5498BE72` _stack) (`HaverestTimer_8_4CBEDCDD4EF9D546C3314B9C8C4D3794` _haveresttimer) (`DamageAmount_16_08AB22364C359D83888980B8C05B9EEA` _damageamount)) (break `/Game/01_Blueprints/Items/Structure/Stc_Child_Item_Values` (`.Values_12_3CB50DDA4AFF9573FB8EAB88122D203F` (break `/Game/01_Blueprints/Items/Structure/Stc_ItemsData` _returnvalue))))
      (set `self.DispenderCount` _dispender)
      (set `self.Stack` _stack)
      (set `self.HaverestTimer` _haveresttimer)
      (set `self.DamageAmount` _damageamount))))

(event `/Game/01_Blueprints/Interface/IF_Interactable.Interact`
  (params (Character :type "Character Object Reference"))
  (bind (_needitem_datatable _needitem_rowname) (break `DataTableRowHandle` (`self.NeedItem`)))
  (bind _skeletalmesh (`self.SkeletalMesh`))
  (bind _skeletalmesh_2 (`self.SkeletalMesh`))
  (bind _skeletalmesh_3 (`self.SkeletalMesh`))
  (set `self.Character` Character)
  ; Cheat
  (if (not (`self.IsCheat`))
    (if (and (`self.SurchTool`) (`self.Harvestable`))
      (`FMODBlueprintStatics.PlayEvent2D` "/Game/FMOD/Events/SFX/Dispender/SFX_Dispender_Collect_Bonus.SFX_Dispender_Collect_Bonus")
      (set `self.Harvestable` false)
      (`|ExecutionSequence`
        (:`then_0`
          ; Interact Animation
          (`SkeletalMeshComponent.PlayAnimation` _skeletalmesh (`self.Anim_Interact`) false)
          (`SkeletalMeshComponent.SetPlayRate` _skeletalmesh 1.0)
          (`KismetSystemLibrary.Delay` 1.0)
          ; Haverastable Time Animation
          (`SkeletalMeshComponent.PlayAnimation` _skeletalmesh_2 (`self.Anim_HarvestableTime`) false)
          (`SkeletalMeshComponent.SetPlayRate` _skeletalmesh_2 (/ (/ (`self.HaverestTimer`) 10.0) 60.0))
          (`KismetSystemLibrary.Delay` (* (`self.HaverestTimer`) 60.0))
          ; Haverastable Animation
          (`FMODBlueprintStatics.PlayEventAtLocation` "/Game/FMOD/Events/SFX/Dispender/SFX_Dispender_Collect_Happy.SFX_Dispender_Collect_Happy" (`self.GetTransform`))
          (`SkeletalMeshComponent.PlayAnimation` _skeletalmesh_3 (`self.Anim_Harvestable`) false)
          (`SkeletalMeshComponent.SetPlayRate` _skeletalmesh_3 1.0)
          (`KismetSystemLibrary.Delay` 1.0)
          (set `self.Harvestable` true))
        (:`then_1`
          (`/Game/01_Blueprints/SaveGame/LS_SaveGame_Character.AddCount` (`/Game/01_Blueprints/Library/FL_Utils.LS_SaveGame_Character`) (`self.ItemName`) (`self.DispenderCount`) (`self.Stack`))
          (`/Game/04_UI/Widgets/AWB_HUD.Damage` (`/Game/01_Blueprints/Library/FL_Utils.LS_HUD`) (`KismetMathLibrary.Conv_IntToDouble` (`self.DamageAmount`)))))
      (else
        (`KismetSystemLibrary.PrintString` (`KismetStringLibrary.Conv_NameToString` _needitem_rowname))))
    (else
      (`self.Cheat`))))

(event `Cheat`
  (bind _skeletalmesh (`self.SkeletalMesh`))
  (bind _skeletalmesh_2 (`self.SkeletalMesh`))
  (bind _skeletalmesh_3 (`self.SkeletalMesh`))
  (if (`self.Harvestable`)
    (set `self.Harvestable` false)
    (`FMODBlueprintStatics.PlayEvent2D` "/Game/FMOD/Events/SFX/Dispender/SFX_Dispender_Collect_Bonus.SFX_Dispender_Collect_Bonus")
    (`|ExecutionSequence`
      (:`then_0`
        ; Interact Animation
        (`SkeletalMeshComponent.PlayAnimation` _skeletalmesh_3 (`self.Anim_Interact`) false)
        (`SkeletalMeshComponent.SetPlayRate` _skeletalmesh_3 1.0)
        (`KismetSystemLibrary.Delay` 1.0)
        ; Haverastable Time Animation
        (`SkeletalMeshComponent.PlayAnimation` _skeletalmesh (`self.Anim_HarvestableTime`) false)
        (`SkeletalMeshComponent.SetPlayRate` _skeletalmesh 1.0)
        (`KismetSystemLibrary.Delay` 1.0)
        ; Haverastable Animation
        (`FMODBlueprintStatics.PlayEventAtLocation` "/Game/FMOD/Events/SFX/Dispender/SFX_Dispender_Collect_Happy.SFX_Dispender_Collect_Happy" (`self.GetTransform`))
        (`SkeletalMeshComponent.PlayAnimation` _skeletalmesh_2 (`self.Anim_Harvestable`) false)
        (`SkeletalMeshComponent.SetPlayRate` _skeletalmesh_2 1.0)
        (`KismetSystemLibrary.Delay` 1.0)
        (set `self.Harvestable` true))
      (:`then_1`
        (`/Game/01_Blueprints/SaveGame/LS_SaveGame_Character.AddCount` (`/Game/01_Blueprints/Library/FL_Utils.LS_SaveGame_Character`) (`self.ItemName`) (`self.DispenderCount`) (`self.Stack`))
        (`/Game/04_UI/Widgets/AWB_HUD.Damage` (`/Game/01_Blueprints/Library/FL_Utils.LS_HUD`) (`KismetMathLibrary.Conv_IntToDouble` (`self.DamageAmount`)))))))

(fn `InteractOverlap`
  (returns (Enumirator :type "/Game/01_Blueprints/Enumiration/E_InteractTyp Enum"))
  (return "NewEnumerator3"))

(fn `SurchTool`
  (returns (ReturnValue :type Boolean))
  (locals (Found :type Boolean :default false))
  (bind (_needitem_datatable _needitem_rowname) (break `DataTableRowHandle` (`self.NeedItem`)))
  (`/Engine/EditorBlueprintResources/StandardMacros.IsValid` _needitem_datatable
    (:`Is Valid`
      (bind _output_get (set `local.Found` (not (== (`KismetArrayLibrary.Array_Find` (`/Game/01_Blueprints/Library/FL_Utils.LS_Blueprints`) _needitem_rowname) -1)))))
    (:`Is Not Valid`
      (set `local.Found` true)))
  (return _output_get))

(fn `UserConstructionScript`)