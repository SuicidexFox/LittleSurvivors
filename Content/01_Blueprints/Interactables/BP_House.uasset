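; BP_House is an interactable house where the player customizes their character's skin, hair, face and clothing on a preview rig.
; Interacting loads the saved look, fades the camera to the house view and opens its UI.
; Items sent to it are looked up in DT_Items and applied by clothing type, with jumpsuits and separate over/underwear clearing each other.
; Leaving saves the outfit, notifies the character and fades the view back.
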(event `SetupUserAssets`
  (bind _sg_character (`/Game/01_Blueprints/Library/FL_Utils.LS_SaveGame_Character`))
  (`PrimitiveComponent.SetMaterial` (`self.SKM_Rig`) 0 (`/Game/01_Blueprints/SaveGame/LS_SaveGame_Character.SkinColor` _sg_character))
  (`StaticMeshComponent.SetStaticMesh` (`self.Hair`) (`/Game/01_Blueprints/SaveGame/LS_SaveGame_Character.Hair` _sg_character))
  (`StaticMeshComponent.SetStaticMesh` (`self.Face`) (`/Game/01_Blueprints/SaveGame/LS_SaveGame_Character.Face` _sg_character))
  (`ChaosClothComponent.SetAsset` (`self.Overware`) (`/Game/01_Blueprints/SaveGame/LS_SaveGame_Character.Overware` _sg_character))
  (`ChaosClothComponent.SetAsset` (`self.Underware`) (`/Game/01_Blueprints/SaveGame/LS_SaveGame_Character.Underware` _sg_character))
  (`ChaosClothComponent.SetAsset` (`self.Jumpsuit`) (`/Game/01_Blueprints/SaveGame/LS_SaveGame_Character.Jumpsuit` _sg_character)))

(event `/Game/01_Blueprints/Interface/IF_Interactable.Interact`
  (params (Character :type "Character Object Reference"))
  (bind _returnvalue (`GameplayStatics.GetPlayerController` 0))
  (bind _fadeduration (`self.FadeDuration`))
  (bind _playercameramanager (`PlayerController.PlayerCameraManager` _returnvalue))
  ; Interact
  (bind _output_get (set `self.Character` Character))
  (`self.SetupUserAssets`)
  (set `MovementComponent.Velocity` (0.0 0.0 0.0) (`Character.CharacterMovement` _output_get))
  (`PlayerCameraManager.StartCameraFade` :`self` _playercameramanager :`ToAlpha` 1.0 :`Duration` _fadeduration)
  (`KismetSystemLibrary.Delay` _fadeduration)
  (`PlayerController.SetViewTargetWithBlend` _returnvalue self 0.0 "VTBlend_Linear" 0.0 true)
  (`PlayerCameraManager.StartCameraFade` :`self` _playercameramanager :`FromAlpha` 1.0 :`Duration` _fadeduration)
  (`/Game/01_Blueprints/LS_UserInterface.SetupInteractables` (`/Game/01_Blueprints/Library/FL_Utils.LS_UserInterface`) self (`self.Activatable Widget Class`)))

(event `self.LeaveInteract`
  (bind _returnvalue (`GameplayStatics.GetPlayerController` 0))
  (bind _character (`self.Character`))
  (bind _fadeduration (`self.FadeDuration`))
  (bind _playercameramanager (`PlayerController.PlayerCameraManager` _returnvalue))
  ; Leave
  (`self.SaveCloth`)
  (`PlayerCameraManager.StartCameraFade` :`self` _playercameramanager :`ToAlpha` 1.0 :`Duration` _fadeduration)
  (message `/Game/01_Blueprints/Interface/IF_Character.ChangeItems` _character)
  (`KismetSystemLibrary.Delay` _fadeduration)
  (`PlayerController.SetViewTargetWithBlend` _returnvalue _character 0.0 "VTBlend_Linear" 0.0 true)
  (`PlayerCameraManager.StartCameraFade` :`self` _playercameramanager :`FromAlpha` 1.0 :`Duration` _fadeduration))

(event `/Game/01_Blueprints/Interface/IF_Interactable.SendItemToBP`
  (params (ItemName :type Name))
  (bind _returnvalue (`|GetDataTableRow` "/Game/01_Blueprints/Items/DT_Items.DT_Items" ItemName)
    (:`then`
      (`FMODBlueprintStatics.PlayEvent2D` "/Game/FMOD/Events/SFX/ButtonShop/SFX_Buy.SFX_Buy")
      (bind (_clothtyp _material _asset _cloth) (break `/Game/01_Blueprints/Items/Structure/Stc_Child_Item_Cloth` (`.Cloth_15_C20A8C684D2F5F21EEE239B1F7083053` (break `/Game/01_Blueprints/Items/Structure/Stc_ItemsData` _returnvalue))))
      (switch `/Game/01_Blueprints/Enumiration/Enum_ClothTyp` _clothtyp
        (:`NewEnumerator6`
          (bind _output_get (set `self.SkinMaterial` _material))
          (`PrimitiveComponent.SetMaterial` (`self.SKM_Rig`) 0 _output_get))
        (:`NewEnumerator1`
          (`StaticMeshComponent.SetStaticMesh` (`self.Hair`) _asset))
        (:`NewEnumerator0`
          (`StaticMeshComponent.SetStaticMesh` (`self.Face`) _asset))
        (:`NewEnumerator2`
          (`ChaosClothComponent.SetAsset` (`self.Overware`) _cloth)
          (`ChaosClothComponent.SetAsset` (`self.Jumpsuit`) null :!label _label))
        (:`NewEnumerator3`
          (`ChaosClothComponent.SetAsset` (`self.Underware`) _cloth)
          (goto _label))
        (:`NewEnumerator4`
          (`ChaosClothComponent.SetAsset` (`self.Jumpsuit`) _cloth)
          (`ChaosClothComponent.SetAsset` (`self.Underware`) null)
          (`ChaosClothComponent.SetAsset` (`self.Overware`) null))))))

(event `SaveCloth`
  (bind _sg_character (`/Game/01_Blueprints/Library/FL_Utils.LS_SaveGame_Character`))
  (set `/Game/01_Blueprints/SaveGame/LS_SaveGame_Character.SkinColor` (`self.SkinMaterial`) _sg_character)
  (set `/Game/01_Blueprints/SaveGame/LS_SaveGame_Character.Hair` (`StaticMeshComponent.StaticMesh` (`self.Hair`)) _sg_character)
  (set `/Game/01_Blueprints/SaveGame/LS_SaveGame_Character.Face` (`StaticMeshComponent.StaticMesh` (`self.Face`)) _sg_character)
  (set `/Game/01_Blueprints/SaveGame/LS_SaveGame_Character.Overware` (`ChaosClothComponent.GetAsset` (`self.Overware`)) _sg_character)
  (set `/Game/01_Blueprints/SaveGame/LS_SaveGame_Character.Underware` (`ChaosClothComponent.GetAsset` (`self.Underware`)) _sg_character)
  (set `/Game/01_Blueprints/SaveGame/LS_SaveGame_Character.Jumpsuit` (`ChaosClothComponent.GetAsset` (`self.Jumpsuit`)) _sg_character))

(fn `InteractOverlap`
  (returns (Enumirator :type "/Game/01_Blueprints/Enumiration/E_InteractTyp Enum"))
  (return "NewEnumerator1"))

(fn `UserConstructionScript`)