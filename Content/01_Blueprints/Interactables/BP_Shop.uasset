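; Interactable shop that hands the player over to a shop view and UI, with a looping timer that periodically plays its FMOD sound ("Wuff").
; Interact halts and disables the character, blends the camera to the shop, plays an interact animation and passes its activatable widget class to the user interface.
; LeaveInteract plays the exit animation, blends the camera back and re-enables input after a delay matching the blend.
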(event `self.ReceiveBeginPlay`
  (`KismetSystemLibrary.K2_SetTimer` null "Wuff" 10.0 true true))

(event `Wuff`
  (`FMODAudioComponent.Play` (`self.FMODAudio`)))

(event `/Game/01_Blueprints/Interface/IF_Interactable.Interact`
  (params (Character :type "Character Object Reference"))
  (bind _returnvalue (`GameplayStatics.GetPlayerController` 0))
  (bind _output_get (set `self.Character` Character))
  (set `MovementComponent.Velocity` (0.0 0.0 0.0) (`Character.CharacterMovement` _output_get))
  (`self.DisableInput` _output_get _returnvalue)
  (`PlayerController.SetViewTargetWithBlend` _returnvalue self 1.0 "VTBlend_Linear" 0.0 true)
  (`SkeletalMeshComponent.PlayAnimation` (`self.SkeletalMesh`) (`self.AnimInteracte`) false)
  (`/Game/01_Blueprints/LS_UserInterface.SetupInteractables` (`/Game/01_Blueprints/Library/FL_Utils.LS_UserInterface`) self (`self.Activatable Widget Class`)))

(event `/Game/01_Blueprints/Interface/IF_Interactable.LeaveInteract`
  (bind _returnvalue (`GameplayStatics.GetPlayerController` 0))
  (bind _character (`self.Character`))
  (`SkeletalMeshComponent.PlayAnimation` (`self.SkeletalMesh`) (`self.AnimLeaveInteract`) false)
  (`PlayerController.SetViewTargetWithBlend` _returnvalue _character 1.0 "VTBlend_Linear" 0.0 true)
  (`KismetSystemLibrary.Delay` 1.0)
  (`self.EnableInput` _character _returnvalue))

(fn `InteractOverlap`
  (returns (Enumirator :type "/Game/01_Blueprints/Enumiration/E_InteractTyp Enum"))
  (return "NewEnumerator5"))

(fn `UserConstructionScript`)