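; BP_Sandbox is an interactable that takes over the player's view when a character interacts with it.
; Interact stops the character, disables its input, blends the camera to itself and hands itself and an activatable widget class to the LSUI interactables setup.
; LeaveInteract blends the view back to the character and restores input after a delay matching the blend.
; InteractOverlap returns a fixed enum value.
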(event `/Game/01_Blueprints/Interface/IF_Interactable.Interact`
  (params (Character :type "Character Object Reference"))
  (bind _returnvalue (`GameplayStatics.GetPlayerController` 0))
  (bind _output_get (set `self.Character` Character))
  (set `MovementComponent.Velocity` (0.0 0.0 0.0) (`Character.CharacterMovement` _output_get))
  (`self.DisableInput` _output_get _returnvalue)
  (`PlayerController.SetViewTargetWithBlend` _returnvalue self 1.0 "VTBlend_Linear" 0.0 true)
  (`/Game/01_Blueprints/LS_UserInterface.SetupInteractables` (`/Game/01_Blueprints/Library/FL_Utils.LS_UI`) self (`self.Activatable Widget Class`)))

(event `/Game/01_Blueprints/Interface/IF_Interactable.LeaveInteract`
  (bind _returnvalue (`GameplayStatics.GetPlayerController` 0))
  (bind _character (`self.Character`))
  (`PlayerController.SetViewTargetWithBlend` _returnvalue _character 1.0 "VTBlend_Linear" 0.0 true)
  (`KismetSystemLibrary.Delay` 1.0)
  (`self.EnableInput` _character _returnvalue))

(fn `InteractOverlap`
  (returns (Enumirator :type "/Game/01_Blueprints/Enumiration/E_InteractTyp Enum"))
  (return "NewEnumerator2"))

(fn `UserConstructionScript`)