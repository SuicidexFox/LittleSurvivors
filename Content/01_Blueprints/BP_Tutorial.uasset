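; BP_Tutorial is an actor that runs the introductory tutorial, showing HUD prompts for movement, running, camera rotation, zoom, farming and clothing changes in sequence.
; Each movement and camera step re-checks the player character's velocity or camera input every tick through DelayUntilNextTick loops, then removes its prompt and starts the next.
; The farming and change-cloth prompts advance on fixed timers, after which the actor destroys itself.
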(event `self.ReceiveBeginPlay`
  (`/Game/04_UI/Widgets/AWB_HUD.PushTutorial` (`/Game/01_Blueprints/Library/FL_Utils.LS_UserHUD`) "/Game/04_UI/Widgets/Tutorial/Tutorial_Movement.Tutorial_Movement_C")
  (bind _asls_character (cast `/Game/01_Blueprints/LS_Character` (`GameplayStatics.GetPlayerCharacter` 0)))
  (bind _output_get (set `self.As LS Character` _asls_character))
  (if (> (`KismetMathLibrary.VSizeXY` (`MovementComponent.Velocity` (`Character.CharacterMovement` _output_get))) 50.0) :!label _label
    (`/Game/04_UI/Widgets/AWB_HUD.RemoveTutorial` (`/Game/01_Blueprints/Library/FL_Utils.LS_UserHUD`))
    (`self.Run`)
    (else
      (`KismetSystemLibrary.DelayUntilNextTick`)
      (goto _label))))

(event `Run`
  (`/Game/04_UI/Widgets/AWB_HUD.PushTutorial` (`/Game/01_Blueprints/Library/FL_Utils.LS_UserHUD`) "/Game/04_UI/Widgets/Tutorial/Tutorial_Run.Tutorial_Run_C")
  (if (> (`KismetMathLibrary.VSizeXY` (`MovementComponent.Velocity` (`Character.CharacterMovement` (`self.As LS Character`)))) 260.0) :!label _label_2
    (`/Game/04_UI/Widgets/AWB_HUD.RemoveTutorial` (`/Game/01_Blueprints/Library/FL_Utils.LS_UserHUD`))
    (`self.CameraRotation`)
    (else
      (`KismetSystemLibrary.DelayUntilNextTick`)
      (goto _label_2))))

(event `CameraRotation`
  (`/Game/04_UI/Widgets/AWB_HUD.PushTutorial` (`/Game/01_Blueprints/Library/FL_Utils.LS_UserHUD`) "/Game/04_UI/Widgets/Tutorial/Tutorial_Camera.Tutorial_Camera_C")
  (if (!= (`/Game/01_Blueprints/LS_Character.CamRotationActionValue` (`self.As LS Character`)) 0.0) :!label _label_3
    (`/Game/04_UI/Widgets/AWB_HUD.RemoveTutorial` (`/Game/01_Blueprints/Library/FL_Utils.LS_UserHUD`))
    (`self.CameraZoom`)
    (else
      (`KismetSystemLibrary.DelayUntilNextTick`)
      (goto _label_3))))

(event `CameraZoom`
  (`/Game/04_UI/Widgets/AWB_HUD.PushTutorial` (`/Game/01_Blueprints/Library/FL_Utils.LS_UserHUD`) "/Game/04_UI/Widgets/Tutorial/Tutorial_Zoom.Tutorial_Zoom_C")
  (if (!= (`/Game/01_Blueprints/LS_Character.CamZoomActionValue` (`self.As LS Character`)) 0.0) :!label _label_4
    (`/Game/04_UI/Widgets/AWB_HUD.RemoveTutorial` (`/Game/01_Blueprints/Library/FL_Utils.LS_UserHUD`))
    (`self.Farming`)
    (else
      (`KismetSystemLibrary.DelayUntilNextTick`)
      (goto _label_4))))

(event `Farming`
  (bind _hud (`/Game/01_Blueprints/Library/FL_Utils.LS_UserHUD`))
  (bind _hud_2 (`/Game/01_Blueprints/Library/FL_Utils.LS_UserHUD`))
  (`/Game/04_UI/Widgets/AWB_HUD.PushTutorial` _hud_2 "/Game/04_UI/Widgets/Tutorial/Tutorial_Farming.Tutorial_Farming_C")
  (`KismetSystemLibrary.Delay` 10.0)
  (`/Game/04_UI/Widgets/AWB_HUD.RemoveTutorial` _hud)
  (`/Game/04_UI/Widgets/AWB_HUD.PushTutorial` _hud_2 "/Game/04_UI/Widgets/Tutorial/Tutorial_ChangeCloth.Tutorial_ChangeCloth_C")
  (`KismetSystemLibrary.Delay` 10.0)
  (`/Game/04_UI/Widgets/AWB_HUD.RemoveTutorial` _hud)
  (`self.K2_DestroyActor`))

(fn `UserConstructionScript`)