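; LS_UI manages the game's on-screen UI, creating one overlay at BeginPlay and pushing the player HUD onto it.
; HUD, menu, inventory and interactable screens use separate activatable widget stacks in the overlay.
; Pause and inventory toggle via FlipFlops with background blur, with pause also pausing the game.
; Helpers switch input mode and cursor between game and UI, and leaving an interactable notifies its stored actor.
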(event `self.ReceiveBeginPlay`
  (bind _returnvalue (`|CreateWidget` "/Game/UI/CUW_Overlay.CUW_Overlay_C" (`GameplayStatics.GetPlayerController` 0)))
  (bind _output_get (set `self.UI Overlay` _returnvalue))
  (`UserWidget.AddToViewport` _output_get 0)
  (`self.SetupPlayerHUD`))

(event `SetupInteractables`
  (params (ActivatableWidgetClass :type "CommonActivatableWidget Class Reference") (BP :type "Actor Object Reference"))
  (set `self.CurrentActor` BP)
  (`CommonActivatableWidgetContainerBase.BP_AddWidget` (`/Game/UI/CUW_Overlay.InteractableStack` (`self.UI Overlay`)) ActivatableWidgetClass)
  (`self.UI`))

(event `LeaveInteractable`
  (message `/Game/Blueprints/Interface/IF_Interactable.LeaveInteract` (`self.CurrentActor`))
  (`CommonActivatableWidgetContainerBase.ClearWidgets` (`/Game/UI/CUW_Overlay.InteractableStack` (`self.UI Overlay`)))
  (`self.GameMode`))

(event `Setup Pause`
  (bind _ui_overlay (`self.UI Overlay`))
  (bind _menustack (`/Game/UI/CUW_Overlay.MenuStack` _ui_overlay))
  (`/Engine/EditorBlueprintResources/StandardMacros.FlipFlop`
    (:`A`
      (`GameplayStatics.SetGamePaused` true)
      (`/Game/UI/CUW_Overlay.BlurToggle` _ui_overlay "Visible")
      (`CommonActivatableWidgetContainerBase.BP_AddWidget` _menustack "/Game/UI/Menu/AWB_Pause.AWB_Pause_C")
      (`self.UI`))
    (:`B`
      (`GameplayStatics.SetGamePaused` false)
      (`/Game/UI/CUW_Overlay.BlurToggle` _ui_overlay "Hidden")
      (`CommonActivatableWidgetContainerBase.ClearWidgets` _menustack)
      (`self.GameMode`))))

(fn `GameMode`
  (bind _returnvalue (`GameplayStatics.GetPlayerController` 0))
  (`WidgetBlueprintLibrary.SetInputMode_GameOnly` _returnvalue)
  (set `PlayerController.bShowMouseCursor` false _returnvalue))

(fn `InventoryToggle`
  (bind _ui_overlay (`self.UI Overlay`))
  (bind _inventorystack (`/Game/UI/CUW_Overlay.InventoryStack` _ui_overlay))
  (`/Engine/EditorBlueprintResources/StandardMacros.FlipFlop`
    (:`A`
      (`/Game/UI/CUW_Overlay.BlurToggle` _ui_overlay "Visible")
      (`CommonActivatableWidgetContainerBase.BP_AddWidget` _inventorystack "/Game/UI/AWB_Inventory.AWB_Inventory_C")
      (`self.UI`))
    (:`B`
      (`/Game/UI/CUW_Overlay.BlurToggle` _ui_overlay "Hidden")
      (`CommonActivatableWidgetContainerBase.ClearWidgets` _inventorystack)
      (`self.GameMode`))))

(fn `SetupMainMenu`
  (bind _returnvalue (`CommonActivatableWidgetContainerBase.BP_AddWidget` (`/Game/UI/CUW_Overlay.MenuStack` (`self.UI Overlay`)) "/Game/UI/Menu/AWB_MainMenu.AWB_MainMenu_C"))
  (set `self.MainMenu` _returnvalue)
  (`self.GameMode`))

(fn `SetupPlayerHUD`
  (bind _returnvalue (`CommonActivatableWidgetContainerBase.BP_AddWidget` (`/Game/UI/CUW_Overlay.HUDStack` (`self.UI Overlay`)) "/Game/UI/AWB_HUD.AWB_HUD_C"))
  (set `self.HUD` _returnvalue)
  (`self.GameMode`))

(fn `UI`
  (bind _returnvalue (`GameplayStatics.GetPlayerController` 0))
  (`WidgetBlueprintLibrary.SetInputMode_UIOnlyEx` _returnvalue null)
  (set `PlayerController.bShowMouseCursor` true _returnvalue))

(fn `UserConstructionScript`)