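; Player character with camera-relative movement, running, stepped camera rotation, zoom and interaction with overlapped actors.
; Rotation input steps a target yaw that steers movement and that the actor eases toward each tick, while the spring arm eases to the zoom length, deriving pitch from it.
; Movement input updates a smoothed Direction from velocity relative to actor facing.
; Overlaps track the current interactable for HUD prompts and IF_Interactable messages; interacting zeroes velocity.
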(event `self.ReceiveBeginPlay`)

(event `self.ReceiveTick`
  (params (DeltaSeconds :type "Float (single-precision)"))
  (`self.UpdateYaw`)
  (`self.UpdateCameraZoom`))

(event `self.ReceiveActorEndOverlap`
  (params (OtherActor :type "Actor Object Reference"))
  ;[0.4678 0.1559 0.006512 0.502] Interactables/Switch Image
  (set `self.CurrentInteractable` null)
  (`/Game/UI/AWB_HUD.SetInteractImage` (`/Game/Blueprints/Library/FL_Utils.LS_HUD`) (stale `self.ReceiveActorBeginOverlap` _enumirator) (`KismetSystemLibrary.IsValid` (`self.CurrentInteractable`)) :!label _label))

(event `EnhancedInput|/Game/Blueprints/Inputs/IA_Move`
  (params (ActionValue :type "Vector2D Structure") (ElapsedSeconds :type "Float (double-precision)") (TriggeredSeconds :type "Float (double-precision)") (InputAction :type "InputAction Object Reference" :default "/Game/Blueprints/Inputs/IA_Move.IA_Move"))
  ;[0.03646 1 0.8866] Movement
  (:`Triggered`
    (`self.AddMovementInput` (`KismetMathLibrary.GetForwardVector` (`self.Yaw Rotation`)) ActionValue_X)
    (`self.AddMovementInput` (`KismetMathLibrary.GetRightVector` (`self.Yaw Rotation`)) ActionValue_Y)
    (`self.RotationToMovement`)))

(event `self.ReceiveActorBeginOverlap`
  (params (OtherActor :type "Actor Object Reference"))
  ;[0.4678 0.1559 0.006512 0.502] Interactables/Switch Image
  (bind _output_get (set `self.CurrentInteractable` OtherActor))
  (if (and (`KismetSystemLibrary.IsValid` _output_get) (`KismetSystemLibrary.DoesImplementInterface` OtherActor "/Game/Blueprints/Interface/IF_Interactable.IF_Interactable_C"))
    (bind _enumirator (message `/Game/Blueprints/Interface/IF_Interactable.InteractOverlap` (`self.CurrentInteractable`)))
    (goto _label)))

(event `EnhancedInput|/Game/Blueprints/Inputs/IA_CamRotation`
  (params (ActionValue :type "Float (double-precision)") (ElapsedSeconds :type "Float (double-precision)") (TriggeredSeconds :type "Float (double-precision)") (InputAction :type "InputAction Object Reference" :default "/Game/Blueprints/Inputs/IA_CamRotation.IA_CamRotation"))
  (bind (_yaw_rotation_roll _yaw_rotation_pitch _yaw_rotation_yaw) (`KismetMathLibrary.BreakRotator` (`self.Yaw Rotation`)))
  ;[0.03646 1 0.8866] Movement
  (:`Started`
    (set `self.Yaw Rotation` (`KismetMathLibrary.MakeRotator` _yaw_rotation_roll _yaw_rotation_pitch (+ _yaw_rotation_yaw (* ActionValue (`self.RotationStep`)))))))

(event `EnhancedInput|/Game/Blueprints/Inputs/IA_Interact`
  (params (ActionValue :type Boolean) (ElapsedSeconds :type "Float (double-precision)") (TriggeredSeconds :type "Float (double-precision)") (InputAction :type "InputAction Object Reference" :default "/Game/Blueprints/Inputs/IA_Interact.IA_Interact"))
  ;[0.4678 0.1559 0.006512 0.502] Interactables/Switch Image
  (:`Started`
    (set `MovementComponent.Velocity` (0.0 0.0 0.0) (`self.CharacterMovement`))
    (message `/Game/Blueprints/Interface/IF_Interactable.Interact` (`self.CurrentInteractable`) self)))

(event `EnhancedInput|/Game/Blueprints/Inputs/IA_CamLenght`
  (params (ActionValue :type "Float (double-precision)") (ElapsedSeconds :type "Float (double-precision)") (TriggeredSeconds :type "Float (double-precision)") (InputAction :type "InputAction Object Reference" :default "/Game/Blueprints/Inputs/IA_CamLenght.IA_CamLenght"))
  ;[0.03646 1 0.8866] Movement
  (:`Triggered`
    (set `self.CurrentZoom` (+ (* ActionValue (`self.ZoomStep`)) (`KismetMathLibrary.FClamp` (`self.CurrentZoom`) 100.0 300.0)))))

(event `EnhancedInput|/Game/Blueprints/Inputs/IA_Run`
  (params (ActionValue :type Boolean) (ElapsedSeconds :type "Float (double-precision)") (TriggeredSeconds :type "Float (double-precision)") (InputAction :type "InputAction Object Reference" :default "/Game/Blueprints/Inputs/IA_Run.IA_Run"))
  (bind _charactermovement (`self.CharacterMovement`))
  (bind _runspeed (`self.RunSpeed`))
  (bind _maxwalkspeed (`CharacterMovementComponent.MaxWalkSpeed` _charactermovement))
  ;[0.03646 1 0.8866] Movement
  (:`Started`
    (set `CharacterMovementComponent.MaxWalkSpeed` (* _maxwalkspeed _runspeed) _charactermovement)
    (set `self.Run` true))
  (:`Completed`
    (set `CharacterMovementComponent.MaxWalkSpeed` (/ _maxwalkspeed _runspeed) _charactermovement)
    (set `self.Run` false)))

(fn `RotationToMovement`
  (bind (_returnvalue_location _returnvalue_rotation) (`KismetMathLibrary.BreakTransform` (`SkinnedMeshComponent.GetBoneTransform` (`self.Mesh`) "Root" "RTS_ParentBoneSpace")))
  (bind (_returnvalue_roll _returnvalue_pitch _returnvalue_yaw) (`KismetMathLibrary.BreakRotator` (`KismetMathLibrary.RInterpTo` _returnvalue_rotation (`KismetMathLibrary.RLerp` _returnvalue_rotation (`KismetMathLibrary.MakeRotator` 0.0 0.0 (`KismetAnimationLibrary.CalculateDirection` (`MovementComponent.Velocity` (`self.CharacterMovement`)) (`self.K2_GetActorRotation`))) 1.0 true) (`GameplayStatics.GetWorldDeltaSeconds`) 10.0)))
  (set `self.Direction` _returnvalue_yaw))

(fn `UpdateCameraZoom`
  (bind _output_get (set `SpringArmComponent.TargetArmLength` (`KismetMathLibrary.FInterpTo` (`SpringArmComponent.TargetArmLength` (`self.SpringArm`)) (`self.CurrentZoom`) (`GameplayStatics.GetWorldDeltaSeconds`) (`self.ZoomSpeed`)) (`self.SpringArm`)))
  (`SceneComponent.K2_SetRelativeRotation` (`self.SpringArm`) (`KismetMathLibrary.RInterpTo` (`SceneComponent.RelativeRotation` (`self.SpringArm`)) (`KismetMathLibrary.MakeRotator` 0.0 (/ _output_get -10.0)) (`GameplayStatics.GetWorldDeltaSeconds`) (`self.ZoomSpeed`)) false false))

(fn `UpdateYaw`
  (`self.K2_SetActorRotation` (`KismetMathLibrary.RInterpTo` (`self.K2_GetActorRotation`) (`self.Yaw Rotation`) (`GameplayStatics.GetWorldDeltaSeconds`) (`self.RotationSpeed`))))

(fn `UserConstructionScript`)