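; Utility function library with shortcuts to core LS_ objects and an item requirement check for purchases.
; Getters cast the game instance to reach the character save, its Blueprints and Inventory, or player 0's HUD to reach LS_UI and its HUD.
; ArrayNeedItems compares every array element with each map entry's name and minimum count, printing each result; any mismatch clears CanBuy and breaks the map loop.
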(fn `ArrayNeedItems`
  (params (Array :type "Array of /Game/Items/Structure/Stc_SaveGame_ItemsList Structure") (Map :type "Map of Name to Integer (by ref)"))
  (returns (True :type Boolean))
  (locals (CanBuy :type Boolean :default true))
  (bind (_keypin _valuepin) (`|MapForEach` Map :!label _label)
    (:`then`
      (for _array_element Array
        (bind (_name _count) (break `/Game/Items/Structure/Stc_SaveGame_ItemsList` _array_element))
        (bind _returnvalue (and (== _name _keypin) (>= _count _valuepin)))
        (`KismetSystemLibrary.PrintString` null (`KismetStringLibrary.Conv_BoolToString` _returnvalue))
        (if (not _returnvalue)
          (set `local.CanBuy` false)
          (goto _label :!via `BreakPin`))))
    (:`CompletedPin`
      (return (`local.CanBuy`)))))

(fn `LS_Blueprints`
  (returns (Blueprints :type "Array of Name"))
  (bind _asls_game_instance (cast `/Game/Blueprints/LS_GameInstance` (`GameplayStatics.GetGameInstance` null)))
  (return (`/Game/Blueprints/SaveGame/SG_Character.Blueprints` (`/Game/Blueprints/LS_GameInstance.SG Character` _asls_game_instance))))

(fn `LS_GameInstance`
  (returns (GameInstance :type "/Game/Blueprints/LS_GameInstance Object Reference"))
  (bind _asls_game_instance (cast `/Game/Blueprints/LS_GameInstance` (`GameplayStatics.GetGameInstance` null)))
  (return _asls_game_instance))

(fn `LS_HUD`
  (returns (HUD :type "/Game/UI/AWB_HUD Object Reference"))
  (bind _asls_ui (cast `/Game/Blueprints/LS_UI` (`PlayerController.GetHUD` (`GameplayStatics.GetPlayerController` null))))
  (return (`/Game/Blueprints/LS_UI.HUD` _asls_ui)))

(fn `LS_Inventory`
  (returns (Inventory :type "Array of /Game/Items/Structure/Stc_SaveGame_ItemsList Structure"))
  (bind _asls_game_instance (cast `/Game/Blueprints/LS_GameInstance` (`GameplayStatics.GetGameInstance` null)))
  (return (`/Game/Blueprints/SaveGame/SG_Character.Inventory` (`/Game/Blueprints/LS_GameInstance.SG Character` _asls_game_instance))))

(fn `LS_SaveGame_Character`
  (returns (`SG Character` :type "/Game/Blueprints/SaveGame/SG_Character Object Reference"))
  (bind _asls_game_instance (cast `/Game/Blueprints/LS_GameInstance` (`GameplayStatics.GetGameInstance` null)))
  (return (`/Game/Blueprints/LS_GameInstance.SG Character` _asls_game_instance)))

(fn `LS_UI`
  (returns (UI :type "/Game/Blueprints/LS_UI Object Reference"))
  (bind _asls_ui (cast `/Game/Blueprints/LS_UI` (`PlayerController.GetHUD` (`GameplayStatics.GetPlayerController` null))))
  (return _asls_ui))