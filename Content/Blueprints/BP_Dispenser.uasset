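; BP_Dispenser is an interactable dispenser Blueprint, apparently an unfinished stub, that dispenses nothing yet.
; Its Interact event stores the calling character, then checks that it is harvestable and needs no item, but the passing branch is empty.
; InteractTyp and IsHarvestable expose its interaction type and harvestable flag to callers.
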(event `/Game/Blueprints/Interface/IF_Interactable.Interact`
  (params (Character :type "Character Object Reference"))
  (set `self.CurrentCharacter` Character)
  (if (and (`self.Harvestable`) (== (`self.NeedItrem`) "None"))
    _))

(fn `InteractTyp`
  (returns (Enumirator :type "/Game/Blueprints/Enumiration/E_InteractTyp Enum"))
  (return (`self.Enumirator`)))

(fn `IsHarvestable`
  (returns (Harvestable :type Boolean))
  (return (`self.Harvestable`)))

(fn `UserConstructionScript`)