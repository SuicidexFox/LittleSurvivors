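; BP_Shop is an interactable shop actor that brings up a UI when a character interacts with it.
; Interact stores the character, blends the player's view to the shop, plays the interact animation and passes its activatable widget class to LSUI.
; LeaveInteract blends the view back to the stored character and plays the leave animation.
; InteractOverlap reports a fixed interaction enum value.
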(event `/Game/Blueprints/Interface/IF_Interactable.Interact`
  (params (Character :type "Character Object Reference"))
  (set `self.Character` Character)
  (`PlayerController.SetViewTargetWithBlend` (`GameplayStatics.GetPlayerController` 0) self 1.0 "VTBlend_Linear" 0.0 true)
  (`SkeletalMeshComponent.PlayAnimation` (`self.SkeletalMesh`) (`self.AnimInteracte`) false)
  (`/Game/Blueprints/LS_UI.SetupInteractables` (`/Game/Blueprints/Library/FL_Utils.LS_UI`) self (`self.Activatable Widget Class`)))

(event `/Game/Blueprints/Interface/IF_Interactable.LeaveInteract`
  (`PlayerController.SetViewTargetWithBlend` (`GameplayStatics.GetPlayerController` 0) (`self.Character`) 1.0 "VTBlend_Linear" 0.0 true)
  (`SkeletalMeshComponent.PlayAnimation` (`self.SkeletalMesh`) (`self.AnimLeaveInteract`) false))

(fn `InteractOverlap`
  (returns (Enumirator :type "/Game/Blueprints/Enumiration/E_InteractTyp Enum"))
  (return "NewEnumerator5"))

(fn `UserConstructionScript`)