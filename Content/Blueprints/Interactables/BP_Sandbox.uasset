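; BP_Sandbox is an interactable that shifts the player's view to itself when used.
; On Interact it stores the character, blends the player camera to itself and passes itself with an activatable widget class to the LSUI interactable setup.
; LeaveInteract blends the view back to the stored character, and InteractOverlap returns a fixed enum value.
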(event `/Game/Blueprints/Interface/IF_Interactable.Interact`
  (params (Character :type "Character Object Reference"))
  (set `self.Character` Character)
  (`PlayerController.SetViewTargetWithBlend` (`GameplayStatics.GetPlayerController` 0) self 1.0 "VTBlend_Linear" 0.0 true)
  (`/Game/Blueprints/LS_UI.SetupInteractables` (`/Game/Blueprints/Library/FL_Utils.LS_UI`) self (`self.Activatable Widget Class`)))

(event `/Game/Blueprints/Interface/IF_Interactable.LeaveInteract`
  (`PlayerController.SetViewTargetWithBlend` (`GameplayStatics.GetPlayerController` 0) (`self.Character`) 1.0 "VTBlend_Linear" 0.0 true))

(fn `InteractOverlap`
  (returns (Enumirator :type "/Game/Blueprints/Enumiration/E_InteractTyp Enum"))
  (return "NewEnumerator2"))

(fn `UserConstructionScript`)