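; Game instance Blueprint that owns the user settings and character save objects for the game session.
; On Init it loads each from its save slot or creates a new one; on Shutdown it writes both back.
; Saved audio bus volumes and color vision correction are applied from user settings, but only in the branch where an existing character save loads.
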(event `self.ReceiveInit`
  (`self.SG_UserSettings`)
  (`self.SG_Character`))

(event `SG_UserSettings`
  (bind _returnvalue (`GameplayStatics.DoesSaveGameExist` "UserSettings"))
  (if _returnvalue
    (bind _returnvalue_2 (`GameplayStatics.LoadGameFromSlot` "UserSettings"))
    (bind _assg_user_settings (cast `/Game/Blueprints/SaveGame/SG_UserSettings` _returnvalue_2))
    (set `self.SG UserSettings` _assg_user_settings)
    (else
      (bind _returnvalue_3 (`GameplayStatics.CreateSaveGameObject` "/Game/Blueprints/SaveGame/SG_UserSettings.SG_UserSettings_C"))
      (set `self.SG UserSettings` _returnvalue_3))))

(event `SG_Character`
  (bind _sg_usersettings (`self.SG UserSettings`))
  (bind _returnvalue (`GameplayStatics.DoesSaveGameExist` "Character"))
  (if _returnvalue
    (bind _returnvalue_2 (`GameplayStatics.LoadGameFromSlot` "Character"))
    (bind _assg_character (cast `/Game/Blueprints/SaveGame/SG_Character` _returnvalue_2))
    (set `self.SG Character` _assg_character)
    (`FMODBlueprintStatics.BusSetVolume` "/Game/FMOD/Buses/Master.Master" (`/Game/Blueprints/SaveGame/SG_UserSettings.MasterVolume` _sg_usersettings))
    (`FMODBlueprintStatics.BusSetVolume` "/Game/FMOD/Buses/Master/Music.Music" (`/Game/Blueprints/SaveGame/SG_UserSettings.MusicVolume` _sg_usersettings))
    (`FMODBlueprintStatics.BusSetVolume` "/Game/FMOD/Buses/Master/Ambience.Ambience" (`/Game/Blueprints/SaveGame/SG_UserSettings.AmbienceVolume` _sg_usersettings))
    (`FMODBlueprintStatics.BusSetVolume` "/Game/FMOD/Buses/Master/SFX.SFX" (`/Game/Blueprints/SaveGame/SG_UserSettings.SFXVolume` _sg_usersettings))
    (`FMODBlueprintStatics.BusSetVolume` "/Game/FMOD/Buses/Master/UI.UI" (`/Game/Blueprints/SaveGame/SG_UserSettings.UIVolume` _sg_usersettings))
    (`WidgetBlueprintLibrary.SetColorVisionDeficiencyType` (`/Game/Blueprints/SaveGame/SG_UserSettings.ColorDefMode` _sg_usersettings) 1.0 true)
    (else
      (bind _returnvalue_3 (`GameplayStatics.CreateSaveGameObject` "/Game/Blueprints/SaveGame/SG_Character.SG_Character_C"))
      (set `self.SG Character` _returnvalue_3))))

(event `self.ReceiveShutdown`
  (`GameplayStatics.SaveGameToSlot` (`self.SG UserSettings`) "UserSettings")
  (`GameplayStatics.SaveGameToSlot` (`self.SG Character`) "Character"))