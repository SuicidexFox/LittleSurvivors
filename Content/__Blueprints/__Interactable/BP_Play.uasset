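; BP_Play is a non-harvestable interactable that opens UI and takes over the player's camera view when used.
; On Interact, it pushes a widget chosen by its InteractTyp onto the HUD overlay's PlayerStack and stores it, then blends the view target to itself.
; Only the Tent type maps to a widget (the inventory); the other types, including Play, have none assigned.
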(event `self.Interact`
  (params (Character :type "/Game/__Blueprints/Character_LittleSurvivors Object Reference"))
  (bind _returnvalue (`CommonActivatableWidgetContainerBase.BP_AddWidget` (`/Game/__UI/CUW_Overlay.PlayerStack` (`/Game/__Blueprints/HUD_LittleSurvivors.MyOverlay` (`/Game/__Blueprints/FL_Utils.MyHUD`))) (select `/Game/__Blueprints/__Enumeration/E_InteractTyp` (`self.InteractTyp`) :`NewEnumerator1` "/Game/__UI/AWB_Inventory.AWB_Inventory_C" :!type "CommonActivatableWidget Class Reference")))
  (set `self.UserWidget` _returnvalue)
  (`PlayerController.SetViewTargetWithBlend` (`GameplayStatics.GetPlayerController` 0) self 1.0 "VTBlend_Linear" 0.0 false))

(fn `Interact Typ`
  (returns (Enumirator :type "/Game/__Blueprints/__Enumeration/E_InteractTyp Enum"))
  (return (`self.InteractTyp`)))

(fn `IsHarvestable`
  (returns (Harvestable :type Boolean))
  (return false))

(fn `UserConstructionScript`)