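; BP_Dispenser is an interactable, respawning resource node that adds its data-table item to the player's materials.
; On BeginPlay it loads the item row and spawns sprite billboards at the mesh sockets.
; Interact checks readiness and any required tool (SurchTool tests only the first tool slot), applies HUD damage, and increases the matching GameInstance save material.
; It then hides the billboards and blocks harvesting for the item's timer.
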(event `self.ReceiveBeginPlay`
  (bind (_datatable _rowname) (break `DataTableRowHandle` (`self.Item`)))
  (bind _returnvalue (`|GetDataTableRow` _datatable _rowname)
    (:`then`
      (set `self.ItemInfo` _returnvalue)
      (`self.Billboards`))))

(event `/Game/__Blueprints/__Interface/IF_Interactables.Interact`
  (params (Character :type "/Game/__Blueprints/Character_LittleSurvivors Object Reference"))
  (set `self.Player` Character)
  (if (and (== (`self.NeedTool`) "None") (`self.Harvestable`))
    (set `self.Harvestable` false :!label _label)
    (`/Game/__UI/AWB_Player.Damage` (`/Game/__Blueprints/FL_Utils.MyPlayerHUD`) (/ (`self.Damage`) 100.0))
    (bind _timer (`self.AddInventory`))
    (for _array_element (`self.AllBillboards`)
      (`SceneComponent.SetHiddenInGame` _array_element true false))
    (`KismetSystemLibrary.Delay` _timer)
    (for _array_element_2 (`self.AllBillboards`)
      (`SceneComponent.SetHiddenInGame` _array_element_2 false false))
    (set `self.Harvestable` true)
    (else
      (bind _returnvalue (`self.SurchTool`))
      (if (and _returnvalue (`self.Harvestable`))
        (goto _label)))))

(fn `AddInventory`
  (returns (Timer :type "Float (double-precision)"))
  (bind (_item_datatable _item_rowname) (break `DataTableRowHandle` (`self.Item`)))
  (bind (_dispender _stack _timer) (break `/Game/__Items/Structure/S_Values` (`.Values_24_ABC582BC4A5D90FEE1160DB8ABA7F0D4` (break `/Game/__Items/Structure/S_ItemData` (`self.ItemInfo`)))))
  (bind _material (`/Game/__Blueprints/__SaveGame/SG_Player.Material` (`/Game/__Blueprints/GI_LittleSurvivors.SG Player` (`/Game/__Blueprints/FL_Utils.MyGameInstance`))))
  (for (_array_element _array_index) _material
    (bind (_valid _count _itemdatatable) (break `/Game/__Items/Structure/S_ItemRawList` _array_element))
    (if (== (`.RowName` (break `DataTableRowHandle` _itemdatatable)) _item_rowname)
      (`KismetArrayLibrary.Array_Set` _material _array_index (make `/Game/__Items/Structure/S_ItemRawList` _valid (+ _count _dispender) _itemdatatable))
      (return _timer)))
  (return _timer))

(fn `Billboards`
  (bind _allbillboards (`self.AllBillboards`))
  (for _array_element (`SceneComponent.GetAllSocketNames` (`self.Mesh`))
    (bind _returnvalue (`|AddComponentByClass` "/Script/Engine.BillboardComponent" true (`KismetMathLibrary.MakeTransform` (`SceneComponent.GetSocketLocation` (`self.Mesh`) _array_element) (struct) (* (0.001 0.001 0.001) (`self.BillboardScale`)))))
    (`BillboardComponent.SetSprite` _returnvalue (`self.BillboardSprite`))
    (`KismetArrayLibrary.Array_Add` _allbillboards _returnvalue))
  (for _array_element_2 _allbillboards
    (`SceneComponent.SetHiddenInGame` _array_element_2 false false)))

(fn `Interact Typ`
  (returns (Enumirator :type "/Game/__Blueprints/__Enumeration/E_InteractTyp Enum"))
  (return (cast `/Game/__Blueprints/__Enumeration/E_InteractTyp` (`KismetMathLibrary.Conv_IntToByte` (`KismetMathLibrary.Conv_ByteToInt` (`.Typ_9_5DFEB2454EB1DF36F257DF96D327B028` (break `/Game/__Items/Structure/S_ItemData` (`self.ItemInfo`))))))))

(fn `IsHarvestable`
  (returns (Harvestable :type Boolean))
  (return (`self.Harvestable`)))

(fn `SurchTool`
  (returns (ReturnValue :type Boolean))
  (for _array_element (`/Game/__Blueprints/__SaveGame/SG_Player.Tools` (`/Game/__Blueprints/GI_LittleSurvivors.SG Player` (`/Game/__Blueprints/FL_Utils.MyGameInstance`)))
    (bind (_valid _count _itemdatatable) (break `/Game/__Items/Structure/S_ItemRawList` _array_element))
    (return (and _valid (== (`.RowName` (break `DataTableRowHandle` _itemdatatable)) (`self.NeedTool`))))))

(fn `UserConstructionScript`)