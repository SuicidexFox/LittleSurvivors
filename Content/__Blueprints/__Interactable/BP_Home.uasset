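; BP_Home is an interactable home actor that shifts the player's view to itself and opens an interaction UI.
; Interact stores the character, blends the view target to the actor, and passes a configured activatable widget class and itself to the HUD.
; LeaveInteract blends the view back to the stored character.
; It also reports an interaction type and always returns true for IsHarvestable.
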(event `self.Interact`
  (params (Character :type "/Game/__Blueprints/Character_LittleSurvivors Object Reference"))
  (set `self.Character` Character)
  (`PlayerController.SetViewTargetWithBlend` (`GameplayStatics.GetPlayerController` 0) self 1.0 "VTBlend_Linear" 0.0 true)
  (`/Game/__Blueprints/HUD_LittleSurvivors.SetupInteractables` (`/Game/__Blueprints/FL_Utils.MyHUD`) (`self.Activatable Widget Class`) self))

(event `/Game/__Blueprints/__Interface/IF_Interactables.Leave Interact`
  (`PlayerController.SetViewTargetWithBlend` (`GameplayStatics.GetPlayerController` 0) (`self.Character`) 1.0 "VTBlend_Linear" 0.0 true))

(fn `Interact Typ`
  (returns (Enumirator :type "/Game/__Blueprints/__Enumeration/E_InteractTyp Enum"))
  (return (`self.InteractTyp`)))

(fn `IsHarvestable`
  (returns (Harvestable :type Boolean))
  (return true))

(fn `UserConstructionScript`)